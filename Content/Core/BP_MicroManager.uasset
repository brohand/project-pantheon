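; BP_MicroManager is a manager Blueprint that tracks total, alive and dead players, announcing itself as the server on BeginPlay without an authority check.
; After a short delay it gathers all ThirdPersonCharacter actors into CurrentPlayers and counts them.
; CheckPlayers moves zero-Health players to DeadPlayers and lowers the alive count, but its call in the event graph is unwired.
; Debug prints for PlayerData fields are also unwired.
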(event `self.ReceiveBeginPlay`
  (`KismetSystemLibrary.PrintString` "I am server.")
  (`KismetSystemLibrary.Delay` 1.0)
  (`self.initialCheckPlayers`))

(event `self.ReceiveTick`
  (params (DeltaSeconds :type "Float (single-precision)")))

(fn `checkPlayers`
  (for _array_element (`self.currentPlayers`)
    (if (not (`KismetMathLibrary.Conv_IntToBool` (`/Game/ThirdPersonBP/Blueprints/ThirdPersonCharacter.Health` _array_element)))
      (`/Engine/EditorBlueprintResources/StandardMacros.DecrementInt` (`self.alivePlayerCount`)
        (:`  `
          (`KismetArrayLibrary.Array_Add` (`self.deadPlayers`) _array_element)))))
  (for _array_element_2 (`self.deadPlayers`)
    (`KismetArrayLibrary.Array_RemoveItem` (`self.currentPlayers`) _array_element_2)))

(fn `initialCheckPlayers`
  (bind _outactors (`GameplayStatics.GetAllActorsOfClass` "/Game/ThirdPersonBP/Blueprints/ThirdPersonCharacter.ThirdPersonCharacter_C"))
  (set `self.currentPlayers` _outactors)
  (for _ (`self.currentPlayers`)
    (`/Engine/EditorBlueprintResources/StandardMacros.IncrementInt` (`self.totalPlayerCount`)
      (:`  `
        (`/Engine/EditorBlueprintResources/StandardMacros.IncrementInt` (`self.alivePlayerCount`))))))